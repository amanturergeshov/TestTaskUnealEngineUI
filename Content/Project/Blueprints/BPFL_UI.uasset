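; BPFL_UI is a Blueprint function library that gives access to a player's layered UI, with calls to push, pop and clear widgets by layer name.
; GetPrimaryLayout resolves the primary layout from the player controller's BP_MainHUD.
; Each layer function fetches that layout, checks it is valid and forwards the call to it, including clearing one layer, all layers or all except one.
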(fn `ClearAllLayers`
  (params (OwningPlayer :type "PlayerController Object Reference"))
  (bind _primarylayout (`self.GetPrimaryLayout` OwningPlayer))
  (`/Engine/EditorBlueprintResources/StandardMacros.IsValid` _primarylayout
    (:`Is Valid`
      (`/Game/Project/UI/Layout/WBP_PrimaryLayout.ClearAllLayers` _primarylayout))))

(fn `ClearAllLayersExcept`
  (params (OwningPlayer :type "PlayerController Object Reference") (`Exception Layer Name` :type "GameplayTag Structure"))
  (bind _primarylayout (`self.GetPrimaryLayout` OwningPlayer))
  (`/Engine/EditorBlueprintResources/StandardMacros.IsValid` _primarylayout
    (:`Is Valid`
      (`/Game/Project/UI/Layout/WBP_PrimaryLayout.ClearAllLayersExcept` _primarylayout `Exception Layer Name`))))

(fn `ClearLayer`
  (params (OwningPlayer :type "PlayerController Object Reference") (LayerName :type "GameplayTag Structure"))
  (bind _primarylayout (`self.GetPrimaryLayout` OwningPlayer))
  (`/Engine/EditorBlueprintResources/StandardMacros.IsValid` _primarylayout
    (:`Is Valid`
      (`/Game/Project/UI/Layout/WBP_PrimaryLayout.ClearLayer` _primarylayout LayerName))))

(fn `GetPrimaryLayout`
  (params (OwningPlayerController :type "PlayerController Object Reference"))
  (returns (PrimaryLayout :type "/Game/Project/UI/Layout/WBP_PrimaryLayout Object Reference"))
  (`/Engine/EditorBlueprintResources/StandardMacros.IsValid` OwningPlayerController
    (:`Is Valid`
      (bind _asbp_main_hud (cast `/Game/Project/Blueprints/HUD/BP_MainHUD` (`PlayerController.GetHUD` OwningPlayerController)))
      (return (`/Game/Project/Blueprints/HUD/BP_MainHUD.GetPrimaryLayout` _asbp_main_hud)))))

(fn `PopContentFromLayer`
  (params (OwningPlayer :type "PlayerController Object Reference") (LayerName :type "GameplayTag Structure"))
  (bind _primarylayout (`self.GetPrimaryLayout` OwningPlayer))
  (`/Engine/EditorBlueprintResources/StandardMacros.IsValid` _primarylayout
    (:`Is Valid`
      (`/Game/Project/UI/Layout/WBP_PrimaryLayout.PopContentFromLayer` _primarylayout LayerName))))

(fn `PushContentToLayer`
  (params (OwningPlayer :type "PlayerController Object Reference") (LayerName :type "GameplayTag Structure") (WidgetClass :type "UserWidget Soft Class Reference"))
  (returns (PushedWidget :type "UserWidget Object Reference"))
  (bind _primarylayout (`self.GetPrimaryLayout` OwningPlayer))
  (`/Engine/EditorBlueprintResources/StandardMacros.IsValid` _primarylayout
    (:`Is Valid`
      (bind _widget (`/Game/Project/UI/Layout/WBP_PrimaryLayout.PushContentToLayer` _primarylayout LayerName WidgetClass))
      (return _widget))))